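; BP_Character is a side-scrolling 2D player character with Enhanced Input movement along world X and jumping.
; Every Tick picks the idle or run flipbook from X velocity and rotates the sprite to face travel direction.
; A Z velocity check runs afterwards, overriding that flipbook with jump or fall while airborne.
; A Death event disables input, sets the hit flipbook and prints a message, but does not stop the Tick animation updates.
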(event Custom|Death
  (Input|DisableInput 0)
  (Sprite|SetFlipbook (Variables|Default|GetSprite) "/Game/Sprites/Characters/CharacterOne/Hit/HIT_SPRITE.HIT_SPRITE")
  (Development|PrintString "Muere"))

(event Custom|Update%20Animation%20Z
  ;[0.15 0.15 0.15 0.5] Animacion
  (Math|Float|CompareFloat (.z (Variables|/Script/Engine.MovementComponent|GetVelocity (Variables|Character|GetCharacterMovement))) 0.0
    (:>
      (Sprite|SetFlipbook (Variables|Default|GetSprite) "/Game/Sprites/Characters/CharacterOne/Jump/JUMP_SPRITE.JUMP_SPRITE"))
    (:<
      (Sprite|SetFlipbook (Variables|Default|GetSprite) "/Game/Sprites/Characters/CharacterOne/Fall/FALL_SPRITE.FALL_SPRITE"))))

(event Custom|Update%20Animation%20X
  ;[0.15 0.15 0.15 0.5] Animacion
  (Math|Float|CompareFloat (.x (Variables|/Script/Engine.MovementComponent|GetVelocity (Variables|Character|GetCharacterMovement))) 0.0
    (:>
      (Sprite|SetFlipbook (Variables|Default|GetSprite) "/Game/Sprites/Characters/CharacterOne/Run/RUN_SPRITE.RUN_SPRITE")
      (Transformation|SetRelativeRotation (Variables|Default|GetSprite) "0, 0, 0" false false))
    (:==
      (Sprite|SetFlipbook (Variables|Default|GetSprite) "/Game/Sprites/Characters/CharacterOne/Idle/IDLE_SPRITE.IDLE_SPRITE"))
    (:<
      (Sprite|SetFlipbook (Variables|Default|GetSprite) "/Game/Sprites/Characters/CharacterOne/Run/RUN_SPRITE.RUN_SPRITE")
      (Transformation|SetRelativeRotation (Variables|Default|GetSprite) "0.000000,180.000000,0.000000" false false))))

(event Input|EnhancedActionEvents|EnhancedInputActionIA_Move
  (params (ActionValue :type Float%20%28double-precision%29) (ElapsedSeconds :type Float%20%28double-precision%29) (TriggeredSeconds :type Float%20%28double-precision%29) (InputAction :type Input%20Action%20Object%20Reference :default "/Game/Inputs/IA_Move.IA_Move"))
  ;[0.15 0.15 0.15 0.5] Movimiento
  (Pawn|Input|AddMovementInput "1.000000,0.000000,0.000000" ActionValue false))

(event Input|EnhancedActionEvents|EnhancedInputActionIA_Jump
  (params (ActionValue :type Boolean) (ElapsedSeconds :type Float%20%28double-precision%29) (TriggeredSeconds :type Float%20%28double-precision%29) (InputAction :type Input%20Action%20Object%20Reference :default "/Game/Inputs/IA_Jump.IA_Jump"))
  ;[0.15 0.15 0.15 0.5] Movimiento
  (:Started
    (Character|Jump))
  (:Completed
    (Character|StopJumping)))

(event EventBeginPlay
  ;[0.15 0.15 0.15 0.5] Movimiento
  (Input|AddMappingContext (PlayerController|LocalPlayerSubsystems|GetEnhancedInputLocalPlayerSubsystem (Game|GetPlayerController 0)) "/Game/Inputs/IMC_Base.IMC_Base" 0 "(bIgnoreAllPressedKeysUntilRelease=True,bForceImmediately=False,bNotifyUserSettings=False)"))

(event EventTick
  (params (DeltaSeconds :type Float%20%28single-precision%29))
  ;[0.15 0.15 0.15 0.5] Animacion
  (Utilities|FlowControl|Sequence
    (:then_0
      (CallFunction|UpdateAnimationX))
    (:then_1
      (CallFunction|UpdateAnimationZ))))

(fn ConstructionScript)