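; BP_StartPlatform is the starting platform that kicks off the game and its vertical scrolling when BP_Character overlaps its trigger.
; The first overlap spawns three randomly chosen platforms at stepped heights with random X positions.
; Once started, Tick moves both itself and the BP_Map actor found at BeginPlay along Z by MoveVelocity.
; The platform destroys itself once it drops to a lower Z limit, which also ends its scrolling of the map.
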(event OnComponentBeginOverlap(Trigger)
  (params (OverlappedComponent :type Primitive%20Component%20Object%20Reference) (OtherActor :type Actor%20Object%20Reference) (OtherComp :type Primitive%20Component%20Object%20Reference) (OtherBodyIndex :type Integer) (bFromSweep :type Boolean) (SweepResult :type Hit%20Result%20Structure%20%28by%20ref%29))
  ;[0.15 0.15 0.15 0.5] Start Game
  (Utilities|Casting|CastToBP_Character OtherActor)
  (Variables|Default|SetStarted true)
  (Utilities|FlowControl|DoOnce false
    (:Completed
      (for _index (range 0 2)
        (Game|SpawnActorfromClass (.OutItem (Utilities|Array|Random (Variables|Default|GetPlatform))) (Math|Transform|MakeTransform (Math|Vector|MakeVector (Math|Random|RandomFloatinRange 5e+02 1.11e+03) 0.0 (|((z*234.666667)+70) (Math|Conversions|ToFloat(Integer) _index))) "0, 0, 0" "1.000000,1.000000,1.000000") "Undefined" "MultiplyWithRoot" 0 0)))))

(event EventTick
  (params (DeltaSeconds :type Float%20%28single-precision%29))
  (bind _returnvalue (Transformation|GetActorLocation))
  (bind _movevelocity (Variables|Default|GetMoveVelocity))
  (bind _tilemap (Variables|Default|GetTileMap))
  (bind _returnvalue_2 (Transformation|GetActorLocation _tilemap))
  (bind _returnvalue_3 (* DeltaSeconds _movevelocity))
  ;[0.15 0.15 0.15 0.5] Movement
  (if (Variables|Default|GetStarted)
    (if (<= (.z _returnvalue) -704.0)
      (Actor|DestroyActor)
      (else
        (Utilities|FlowControl|Sequence
          (:then_0
            (Transformation|SetActorLocation (Math|Vector|MakeVector (.x _returnvalue) (.y _returnvalue) (+ _returnvalue_3 (.z _returnvalue))) false false))
          (:then_1
            (Transformation|SetActorLocation (Variables|Default|GetTileMap) (Math|Vector|MakeVector (.x _returnvalue_2) (.y _returnvalue_2) (+ _returnvalue_3 (.z _returnvalue_2))) false false)))))))

(event EventBeginPlay
  ;[0.15 0.15 0.15 0.5] Movement
  (bind _returnvalue (Actor|GetActorOfClass "/Game/Blueprints/BP_Map.BP_Map_C"))
  (Variables|Default|SetTileMap _returnvalue)
  (bind _returnvalue_2 (Actor|GetActorOfClass "/Game/Blueprints/BP_Character.BP_Character_C"))
  (Variables|Default|SetCharacter _returnvalue_2))

(fn ConstructionScript)